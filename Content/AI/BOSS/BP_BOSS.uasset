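; Boss actor that spawns waves of actors once something first overlaps its sphere.
; That overlap sets Begin, letting Tick start a looping timer on BOSSAI, which spawns two monster groups within EnemyAroundArea.
; Projectile overlaps destroy the projectile, subtract fixed HP with no death check, and run a Delay-paced loop spawning within the boss room around a hollow radius.
; That loop's counter never resets, so later hits do not repeat the full batch.
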(event OnComponentBeginOverlap(Sphere)
  (params (OverlappedComponent :type Primitive%20Component%20Object%20Reference) (OtherActor :type Actor%20Object%20Reference) (OtherComp :type Primitive%20Component%20Object%20Reference) (OtherBodyIndex :type Integer) (bFromSweep :type Boolean) (SweepResult :type Hit%20Result%20Structure%20%28by%20ref%29))
  (bind _bossrommarea (Variables|Default|GetBossRommArea))
  (bind (_x _y _z) (Math|Vector|BreakVector _bossrommarea))
  (Variables|Default|SetBegin true)
  (bind _asbp_projectile (Utilities|Casting|CastToBP_Projectile OtherActor))
  (Actor|DestroyActor _asbp_projectile)
  (bind _output_get (Variables|Default|SetHP (- (Variables|Default|GetHP) 2e+01)))
  (Development|PrintString (Utilities|String|ToString(Float) _output_get))
  (Utilities|FlowControl|Delay (Variables|Default|GetSpawnPause) :!label _label)
  (Utilities|SpawnBPinRange "/Game/AI/Virus/BP_White.BP_White_C" _x _y _z (Variables|Default|GetBossRidus))
  (bind _result (Math|Integer|IncrementInt (Variables|Default|GetLoopTimes))
    (:%20%20
      (if (< _result (Variables|Default|GetWhiteNum))
        (goto _label)))))

(event EventTick
  (params (DeltaSeconds :type Float%20%28single-precision%29))
  (Variables|Default|SetDELTATIME (+ DeltaSeconds (Variables|Default|GetDELTATIME)))
  (if (Variables|Default|GetBegin)
    (Utilities|FlowControl|DoOnce false
      (:Completed
        (Utilities|Time|SetTimerbyFunctionName 0 "BOSSAI" (Variables|Default|GetIntervalTime) true)))))

(event EventBeginPlay
  (Variables|Default|SetSpawnLocation (Transformation|GetActorLocation)))

(fn ConstructionScript)

(fn BOSSAI
  (bind _enemyaroundarea (Variables|Default|GetEnemyAroundArea))
  (bind _enemyaroundarea_2 (Variables|Default|GetEnemyAroundArea))
  (bind (_x _y _z) (Math|Vector|BreakVector _enemyaroundarea))
  (bind (_x_2 _y_2 _z_2) (Math|Vector|BreakVector _enemyaroundarea_2))
  (for _index (range 0 (Variables|Default|GetMonstor1Num))
    (Utilities|SpawnBPinRange "/Game/AI/Virus/BP_Virus1_Time.BP_Virus1_Time_C" _x_2 _y_2 _z_2 0.0))
  (for _index_2 (range 0 (Variables|Default|GetMonstor2Num))
    (Utilities|SpawnBPinRange "/Game/AI/Virus/BP_Virus2_big.BP_Virus2_big_C" _x _y _z 0.0)))