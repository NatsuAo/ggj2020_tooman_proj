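; BP_Virus1_Distance is a virus enemy that homes in on the player's FlyingPawn once it comes within a set Distance.
; Each Tick it applies a hundredth of the offset to the player as both a world offset, without sweep, and movement input.
; Hitting the player destroys the virus and reduces player HP.
; BP_Projectile overlaps destroy both projectile and virus, while BP_Projectile_Right overlaps destroy only the projectile.
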(event OnComponentHit(CapsuleComponent)
  (params (HitComponent :type Primitive%20Component%20Object%20Reference) (OtherActor :type Actor%20Object%20Reference) (OtherComp :type Primitive%20Component%20Object%20Reference) (NormalImpulse :type Vector :default "0, 0, 0") (Hit :type Hit%20Result%20Structure%20%28by%20ref%29))
  ;[1 1 1] Hit Player
  (bind _asflying_pawn (Utilities|Casting|CastToFlyingPawn OtherActor))
  (Actor|DestroyActor)
  (Default|ReduceHPbyHit _asflying_pawn))

(event OnComponentBeginOverlap(CapsuleComponent)
  (params (OverlappedComponent :type Primitive%20Component%20Object%20Reference) (OtherActor :type Actor%20Object%20Reference) (OtherComp :type Primitive%20Component%20Object%20Reference) (OtherBodyIndex :type Integer) (bFromSweep :type Boolean) (SweepResult :type Hit%20Result%20Structure%20%28by%20ref%29))
  ;[1 1 1] Hit By Projectle
  (bind _asbp_projectile (Utilities|Casting|CastToBP_Projectile OtherActor)
    (:then
      (Actor|DestroyActor _asbp_projectile)
      (CallFunction|ProjectleHitResult))
    (:CastFailed
      (bind _asbp_projectile_right (Utilities|Casting|CastToBP_Projectile_Right OtherActor))
      (Actor|DestroyActor _asbp_projectile_right))))

(event EventBeginPlay)

(event Collision|EventActorBeginOverlap
  (params (OtherActor :type Actor%20Object%20Reference)))

(event EventTick
  (params (DeltaSeconds :type Float%20%28single-precision%29))
  (bind _returnvalue (Transformation|GetActorLocation))
  (bind _asflying_pawn (Utilities|Casting|CastToFlyingPawn (Game|Player|GetPlayerPawn 0)))
  (if (< (Math|Vector|Distance(Vector) (Transformation|GetActorLocation _asflying_pawn) _returnvalue) (Variables|Default|Getdistance))
    (Transformation|AddActorWorldOffset (/ (- (Transformation|GetActorLocation _asflying_pawn) _returnvalue) 100))
    (Class|PawnMovementComponent|AddInputVector (Variables|Character|GetCharacterMovement) (/ (- (Transformation|GetActorLocation _asflying_pawn) _returnvalue) 100) false)))

(fn ConstructionScript)

(fn UpdateWalkSpeed
  (params (NewWalkSpeed :type Float%20%28single-precision%29))
  (Variables|/Script/Engine.CharacterMovementComponent|SetMaxWalkSpeed (Variables|Character|GetCharacterMovement) NewWalkSpeed))

(fn ProjectleHitResult
  (Actor|DestroyActor))